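; Invader enemy for a shoot-'em-up that moves along the world X axis and awards score when shot.
; Tick calls Play on a timeline, whose track scales MoveSpeed into an unswept world offset on the root each update, without delta-time scaling.
; A Box overlap with a Bullet_Blueprint plays an explosion sound, adds Score to the Shmup_GameStateBase GameScore, then destroys both bullet and invader.
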(event OnComponentBeginOverlap(Box)
  (params (OverlappedComponent :type Primitive%20Component%20Object%20Reference) (OtherActor :type Actor%20Object%20Reference) (OtherComp :type Primitive%20Component%20Object%20Reference) (OtherBodyIndex :type Integer) (bFromSweep :type Boolean) (SweepResult :type Hit%20Result%20Structure%20%28by%20ref%29))
  (Utilities|Casting|CastToBullet_Blueprint OtherActor)
  (Audio|SpawnSound2D "/Game/Audio/Invader_Explosion_01.Invader_Explosion_01" 1.0 1.0 0.0 0)
  (bind _asshmup_game_state_base (Utilities|Casting|CastToShmup_GameStateBase (Game|GetGameState)))
  (Variables|/Game/Blueprints/Shmup_GameStateBase.Shmup_GameStateBase_C|SetGameScore _asshmup_game_state_base (+ (Variables|Default|GetScore) (Variables|/Game/Blueprints/Shmup_GameStateBase.Shmup_GameStateBase_C|GetGameScore _asshmup_game_state_base)))
  (Actor|DestroyActor OtherActor)
  (Actor|DestroyActor (Components|GetOwner (Variables|Default|GetDefaultSceneRoot))))

(event EventBeginPlay)

(event Collision|EventActorBeginOverlap
  (params (OtherActor :type Actor%20Object%20Reference)))

(event EventTick
  (params (DeltaSeconds :type Float%20%28single-precision%29))
  (bind _newtrack_0 (Timeline|Timeline_0 Play)
    (:Update
      (bind _result (Math|Float|NegateFloat (* (Variables|Default|GetMoveSpeed) _newtrack_0))
        (:%20%20
          (Transformation|AddWorldOffset (Variables|Default|GetDefaultSceneRoot) (Math|Vector|MakeVector _result 0.0 0.0) false false))))))

(fn ConstructionScript)
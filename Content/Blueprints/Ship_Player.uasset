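; Player ship Blueprint that moves on axis input and fires bullets.
; Forward input offsets the root along the control rotation's forward vector, and Right input along the root's own right vector.
; Both moves scale by MovementSpeed without delta time or sweep, so they are frame-rate dependent and ignore collision.
; Pressing Shoot spawns a Bullet_Blueprint at the BulletStart transform and plays a 2D laser sound.
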(event EventBeginPlay)

(event Collision|EventActorBeginOverlap
  (params (OtherActor :type Actor%20Object%20Reference)))

(event EventTick
  (params (DeltaSeconds :type Float%20%28single-precision%29)))

(event Input|ActionEvents|InputActionShoot
  (params (Key :type Key%20Structure))
  ;[1 1 1] Shoot
  (:Pressed
    (Game|SpawnActorfromClass "/Game/Blueprints/Bullet_Blueprint.Bullet_Blueprint_C" (Transformation|GetWorldTransform (Variables|Default|GetBullet_Start)) "Undefined" 0 0)
    (Audio|SpawnSound2D "/Game/Audio/Ship_Laser_shoot_02.Ship_Laser_shoot_02" 1.0 1.0 0.0 0)))

(event Input|AxisEvents|InputAxisForward
  (params (AxisValue :type Float%20%28single-precision%29))
  ;[1 1 1] Movement
  (Transformation|AddWorldOffset (Variables|Default|GetDefaultSceneRoot) (* (* (Math|Vector|GetForwardVector (Pawn|GetControlRotation :!class /Script/Engine.Pawn)) AxisValue) (Variables|Default|GetMovementSpeed)) false false))

(event Input|AxisEvents|InputAxisRight
  (params (AxisValue :type Float%20%28single-precision%29))
  ;[1 1 1] Movement
  (Transformation|AddWorldOffset (Variables|Default|GetDefaultSceneRoot) (* (* (Math|Vector|GetRightVector (Variables|Default|GetDefaultSceneRoot)) AxisValue) (Variables|Default|GetMovementSpeed)) false false))

(fn ConstructionScript)